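; First-person player character with directional melee combat, HMD-aware movement, a forward dash on cooldown and a double jump.
; Strike and Block presses sample mouse turn/look input against a threshold to choose one of four directions, then set the matching animation enum.
; Releasing Strike applies radial damage around the player regardless of direction; both releases clear their animation state.
; Dash and double jump use LaunchCharacter, with debug prints throughout.
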(event `InputAxis|MoveForward` :consume false :overrideparent false
  (params (AxisValue :type "Float (single-precision)"))
  ;[1 1 1] FP Movement
  (`self.AddMovementInput` (select `bool` (`HeadMountedDisplayFunctionLibrary.IsHeadMountedDisplayEnabled`) :`false` (`self.GetActorForwardVector`) :`true` (`SceneComponent.GetForwardVector` (`self.FPCamera`))) AxisValue))

(event `InputAxis|Turn`
  (params (AxisValue :type "Float (single-precision)"))
  ;[1 1 1] Turn & LookUp
  (`self.AddControllerYawInput` AxisValue))

(event `InputAxis|MoveRight` :consume false :overrideparent false
  (params (AxisValue :type "Float (single-precision)"))
  ;[1 1 1] FP Movement
  (`self.AddMovementInput` (select `bool` (`HeadMountedDisplayFunctionLibrary.IsHeadMountedDisplayEnabled`) :`false` (`self.GetActorRightVector`) :`true` (`SceneComponent.GetRightVector` (`self.FPCamera`))) AxisValue))

(event `InputAxis|LookUp`
  (params (AxisValue :type "Float (single-precision)"))
  ;[1 1 1] Turn & LookUp
  (`self.AddControllerPitchInput` AxisValue))

(event `InputAction|Strike`
  (params (Key :type "Key Structure"))
  ;[1 1 1] Combat
  (:`Pressed`
    (`self.Mouse Direction Check`)
    (`self.Attack By Direction (Pressed)`)
    (`self.Is Attack`))
  (:`Released`
    (`self.Attack By Direction (Released)`)))

(event `InputAction|Dash`
  (params (Key :type "Key Structure"))
  ;[1 1 1] Dash
  (:`Pressed`
    (if (`self.Dash Reloaded`)
      (`self.LaunchCharacter` (* (`SceneComponent.GetForwardVector` (`self.FPCamera`)) 25000.0))
      (`KismetSystemLibrary.PrintString` "Dashed!" true true (struct :`R` 1.0 :`G` 0.11771 :`A` 1.0))
      (`KismetSystemLibrary.Delay` 0.09)
      (set `self.Dash Reloaded` false)
      (`MovementComponent.StopMovementImmediately` (`self.CharacterMovement`))
      (`KismetSystemLibrary.Delay` 2.0)
      (bind _output_get (set `self.Dash Reloaded` true))
      (`KismetSystemLibrary.PrintString` (`KismetStringLibrary.Concat_StrStr` "Dash Reloaded:" (`KismetStringLibrary.Conv_BoolToString` _output_get)) true true (struct :`R` 0.994792 :`G` 0.091062 :`A` 1.0))
      (else
        (`KismetSystemLibrary.PrintString` "Dash on reload, not yet!")))))

(event `InputAction|Block`
  (params (Key :type "Key Structure"))
  ;[1 1 1] Combat
  (:`Pressed`
    (`self.Block Preparation`)
    (`self.Set Block Anim`))
  (:`Released`
    (`self.Set None Animation`)))

(event `InputAction|Jump`
  (params (Key :type "Key Structure"))
  ;[1 1 1] Double Jump
  (:`Pressed`
    (bind _counter (`/Engine/EditorBlueprintResources/StandardMacros.Do N` 2 :!label _label)
      (:`Exit`
        (switch `int` _counter
          (:`1`
            (`self.Jump`))
          (:`2`
            (`self.LaunchCharacter` (0.0 0.0 750.0))
            (`KismetSystemLibrary.PrintString` "Double jump!" true true (struct :`R` 1.0 :`G` 0.857146 :`A` 1.0))))))))

(event `self.OnLanded`
  (params (Hit :type "HitResult Structure (by ref)"))
  ;[1 1 1] Double Jump
  (goto _label :!via `Reset`))

(event `self.ReceiveBeginPlay`
  (set `self.PlayerCharacter` null))

(event `self.PlayerCharacter.OnTakeAnyDamage`
  (params (DamagedActor :type "Actor Object Reference") (Damage :type "Float (single-precision)") (DamageType :type "DamageType Object Reference") (InstigatedBy :type "Controller Object Reference") (DamageCauser :type "Actor Object Reference"))
  (if true
    _))

(fn `Attack By Direction (Pressed)`
  (switch `/Game/Enum/Enum_StrikeDir` (`self.Strike Direction`)
    (:`NewEnumerator0`
      (bind _output_get (set `self.Strike Anim` "NewEnumerator0"))
      (`KismetSystemLibrary.PrintString` (`|GetEnumeratorNameAsString` _output_get) true true (struct :`R` 1.0 :`B` 0.777277 :`A` 1.0)))
    (:`NewEnumerator1`
      (bind _output_get_2 (set `self.Strike Anim` "NewEnumerator1"))
      (`KismetSystemLibrary.PrintString` (`|GetEnumeratorNameAsString` _output_get_2) true true (struct :`R` 1.0 :`B` 0.777277 :`A` 1.0)))
    (:`NewEnumerator2`
      (bind _output_get_3 (set `self.Strike Anim` "NewEnumerator2"))
      (`KismetSystemLibrary.PrintString` (`|GetEnumeratorNameAsString` _output_get_3) true true (struct :`R` 1.0 :`B` 0.777277 :`A` 1.0)))
    (:`NewEnumerator3`
      (bind _output_get_4 (set `self.Strike Anim` "NewEnumerator3"))
      (`KismetSystemLibrary.PrintString` (`|GetEnumeratorNameAsString` _output_get_4) true true (struct :`R` 1.0 :`B` 0.777277 :`A` 1.0)))
    (:`NewEnumerator4`
      (bind _output_get_5 (set `self.Strike Anim` "NewEnumerator4"))
      (`KismetSystemLibrary.PrintString` (`|GetEnumeratorNameAsString` _output_get_5) true true (struct :`R` 1.0 :`B` 0.777277 :`A` 1.0)))))

(fn `Attack By Direction (Released)`
  (`GameplayStatics.ApplyRadialDamage` :`BaseDamage` 100.0 :`Origin` (`self.K2_GetActorLocation`) :`DamageRadius` 100.0 :`DamageTypeClass` "/Script/Engine.DamageType" :`DamageCauser` null :`InstigatedByController` null :`bDoFullDamage` true)
  (switch `/Game/Enum/Enum_StrikeAnim` (`self.Strike Anim`)
    (:`NewEnumerator0`
      _)
    (:`NewEnumerator1`
      _)
    (:`NewEnumerator2`
      _)
    (:`NewEnumerator3`
      _)
    (:`NewEnumerator4`
      _))
  (set `self.Strike Anim` "NewEnumerator4"))

(fn `Block Preparation`
  (bind _returnvalue (`self.GetInputAxisValue`))
  (bind _returnvalue_2 (`self.GetInputAxisValue`))
  (if (and (`|EnumEquality` (`self.Strike Anim`) "NewEnumerator4") (`|EnumEquality` (`self.Block Anim`) "NewEnumerator4"))
    (if (> _returnvalue_2 (`self.Direction Float`))
      (set `self.Block Direction` "NewEnumerator1")
      (`KismetSystemLibrary.PrintString` "Right Block" true true (struct :`R` 0.101462 :`G` 1.0 :`A` 1.0))
      (elif (< _returnvalue_2 (* -1 (`self.Direction Float`)))
        (set `self.Block Direction` "NewEnumerator2")
        (`KismetSystemLibrary.PrintString` "Left Block" true true (struct :`R` 0.101462 :`G` 1.0 :`A` 1.0))
        (elif (> _returnvalue (`self.Direction Float`))
          (set `self.Block Direction` "NewEnumerator3")
          (`KismetSystemLibrary.PrintString` "Down Block" true true (struct :`R` 0.101462 :`G` 1.0 :`A` 1.0))
          (elif (< _returnvalue (* -1 (`self.Direction Float`)))
            (set `self.Block Direction` "NewEnumerator0")
            (`KismetSystemLibrary.PrintString` "Top Block" true true (struct :`R` 0.101462 :`G` 1.0 :`A` 1.0))))))))

(fn `Mouse Direction Check`
  (bind _returnvalue (`self.GetInputAxisValue`))
  (bind _returnvalue_2 (`self.GetInputAxisValue`))
  (if (and (`|EnumEquality` (`self.Strike Anim`) "NewEnumerator4") (`|EnumEquality` (`self.Block Anim`) "NewEnumerator4"))
    (if (> _returnvalue_2 (`self.Direction Float`))
      (set `self.Strike Direction` "NewEnumerator1")
      (`KismetSystemLibrary.PrintString` "Right Attack")
      (elif (< _returnvalue_2 (* -1 (`self.Direction Float`)))
        (set `self.Strike Direction` "NewEnumerator2")
        (`KismetSystemLibrary.PrintString` "Left Attack")
        (elif (> _returnvalue (`self.Direction Float`))
          (set `self.Strike Direction` "NewEnumerator3")
          (`KismetSystemLibrary.PrintString` "Down Attack")
          (elif (< _returnvalue (* -1 (`self.Direction Float`)))
            (set `self.Strike Direction` "NewEnumerator0")
            (`KismetSystemLibrary.PrintString` "Top Attack")))))))

(fn `Set Block Anim`
  (switch `/Game/Enum/Enum_StrikeAnim` (`self.Block Direction`)
    (:`NewEnumerator0`
      (bind _output_get (set `self.Block Anim` "NewEnumerator0"))
      (`KismetSystemLibrary.PrintString` (`|GetEnumeratorNameAsString` _output_get) true true (struct :`G` 0.28125 :`B` 0.00411 :`A` 1.0)))
    (:`NewEnumerator1`
      (bind _output_get_2 (set `self.Block Anim` "NewEnumerator1"))
      (`KismetSystemLibrary.PrintString` (`|GetEnumeratorNameAsString` _output_get_2) true true (struct :`G` 0.28125 :`B` 0.00411 :`A` 1.0)))
    (:`NewEnumerator2`
      (bind _output_get_3 (set `self.Block Anim` "NewEnumerator2"))
      (`KismetSystemLibrary.PrintString` (`|GetEnumeratorNameAsString` _output_get_3) true true (struct :`G` 0.28125 :`B` 0.00411 :`A` 1.0)))
    (:`NewEnumerator3`
      (bind _output_get_4 (set `self.Block Anim` "NewEnumerator3"))
      (`KismetSystemLibrary.PrintString` (`|GetEnumeratorNameAsString` _output_get_4) true true (struct :`G` 0.28125 :`B` 0.00411 :`A` 1.0)))
    (:`NewEnumerator4`
      (bind _output_get_5 (set `self.Block Anim` "NewEnumerator4"))
      (`KismetSystemLibrary.PrintString` (`|GetEnumeratorNameAsString` _output_get_5) true true (struct :`G` 0.28125 :`B` 0.00411 :`A` 1.0)))))

(fn `Set None Animation`
  (switch `/Game/Enum/Enum_StrikeBlockAnim` (`self.Block Anim`)
    (:`NewEnumerator0`
      _)
    (:`NewEnumerator1`
      _)
    (:`NewEnumerator2`
      _)
    (:`NewEnumerator3`
      _)
    (:`NewEnumerator4`
      _))
  (set `self.Block Anim` "NewEnumerator4"))

(fn `UserConstructionScript`)